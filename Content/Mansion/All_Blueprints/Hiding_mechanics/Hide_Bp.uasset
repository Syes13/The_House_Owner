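; Hide_Bp is a hiding spot that moves the first-person player in or out when interacted with.
; Entering disables the player's collision and movement, then a looping timer at frame delta glides them to PlayerPosition at constant speed, or to ExitPosition when leaving.
; On arrival it clears the timers, calls CallHidingED and flips the player's IsHiding flag, restoring collision and walking on exit.
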(event Custom|Move%20Character
  (bind _playerreference (Variables|Default|GetPlayerReference))
  (Transformation|SetActorTransform _playerreference (Math|Transform|MakeTransform (Math|Interpolation|VInterptoConstant (Transformation|GetActorLocation _playerreference) (Transformation|GetWorldLocation (select (Variables|/Game/FirstPerson/Blueprints/BP_FirstPersonCharacter.BP_FirstPersonCharacter_C|GetIsHiding (Variables|Default|GetPlayerReference)) (Variables|Default|GetExit_Position) (Variables|Default|GetPlayer_Position))) (Utilities|Time|GetWorldDeltaSeconds) 1e+03) "0, 0, 0" "1.000000,1.000000,1.000000"))
  (if (Utilities|Operators|EqualEqual (Transformation|GetWorldLocation (select (Variables|/Game/FirstPerson/Blueprints/BP_FirstPersonCharacter.BP_FirstPersonCharacter_C|GetIsHiding (Variables|Default|GetPlayerReference)) (Variables|Default|GetExit_Position) (Variables|Default|GetPlayer_Position))) (Transformation|GetActorLocation (Variables|Default|GetPlayerReference)) 0.01)
    (Utilities|Time|ClearandInvalidateTimerbyHandle (stale EventInteract _returnvalue_2))
    (Utilities|Time|ClearandInvalidateTimerbyHandle (stale EventInteract _returnvalue))
    (CallFunction|FinishedHiding)))

(event Custom|FinishedHiding
  (bind _playerreference (Variables|Default|GetPlayerReference))
  (Default|CallHidingED)
  (if (Variables|/Game/FirstPerson/Blueprints/BP_FirstPersonCharacter.BP_FirstPersonCharacter_C|GetIsHiding _playerreference)
    (Variables|/Game/FirstPerson/Blueprints/BP_FirstPersonCharacter.BP_FirstPersonCharacter_C|SetIsHiding _playerreference false)
    (Collision|SetActorEnableCollision _playerreference true)
    (Pawn|Components|CharacterMovement|SetMovementMode (Variables|/Script/Engine.Character|GetCharacterMovement _playerreference) "MOVE_Walking" 0)
    (else
      (Variables|/Game/FirstPerson/Blueprints/BP_FirstPersonCharacter.BP_FirstPersonCharacter_C|SetIsHiding _playerreference true))))

(event EventBeginPlay
  (bind _asbp_first_person_character (Utilities|Casting|CastToBP_FirstPersonCharacter (Game|GetPlayerCharacter 0)))
  (Variables|Default|SetPlayerReference _asbp_first_person_character))

(event Collision|EventActorBeginOverlap
  (params (OtherActor :type Actor%20Object%20Reference)))

(event EventTick
  (params (DeltaSeconds :type Float%20%28single-precision%29)))

(event EventInteract
  (bind _playerreference (Variables|Default|GetPlayerReference))
  (if (Variables|/Game/FirstPerson/Blueprints/BP_FirstPersonCharacter.BP_FirstPersonCharacter_C|GetIsHiding (Variables|Default|GetPlayerReference))
    (bind _returnvalue (Utilities|Time|SetTimerbyEvent (delegate Custom|Move%20Character) (Utilities|Time|GetWorldDeltaSeconds) true))
    (else
      (Collision|SetActorEnableCollision _playerreference false)
      (Pawn|Components|CharacterMovement|DisableMovement (Variables|/Script/Engine.Character|GetCharacterMovement _playerreference))
      (bind _returnvalue_2 (Utilities|Time|SetTimerbyEvent (delegate Custom|Move%20Character) (Utilities|Time|GetWorldDeltaSeconds) true)))))

(fn ConstructionScript)