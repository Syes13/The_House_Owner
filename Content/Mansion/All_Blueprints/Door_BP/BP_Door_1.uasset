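; BP_Door_1 is a swinging door that the first-person character can open and close.
; Two trigger boxes set the same 90-degree target rotation and tell BP_FirstPersonCharacter when it can open this door.
; OpenDoor plays or reverses a timeline that lerps DoorN's world rotation between zero and that target.
; Its DoorisCurrentlyOpening guard is only ever set false here, so it does not block repeat calls.
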(event OnComponentBeginOverlap(Box_N)
  (params (OverlappedComponent :type Primitive%20Component%20Object%20Reference) (OtherActor :type Actor%20Object%20Reference) (OtherComp :type Primitive%20Component%20Object%20Reference) (OtherBodyIndex :type Integer) (bFromSweep :type Boolean) (SweepResult :type Hit%20Result%20Structure%20%28by%20ref%29))
  (Variables|Default|SetDooropeningRotator "0.000000,-90.000000,0.000000")
  (bind _asbp_first_person_character (Utilities|Casting|CastToBP_FirstPersonCharacter OtherActor))
  (Default|CanopenDoor _asbp_first_person_character true self))

(event OnComponentBeginOverlap(Box1_N)
  (params (OverlappedComponent :type Primitive%20Component%20Object%20Reference) (OtherActor :type Actor%20Object%20Reference) (OtherComp :type Primitive%20Component%20Object%20Reference) (OtherBodyIndex :type Integer) (bFromSweep :type Boolean) (SweepResult :type Hit%20Result%20Structure%20%28by%20ref%29))
  (Variables|Default|SetDooropeningRotator "0.000000,-90.000000,0.000000")
  (bind _asbp_first_person_character (Utilities|Casting|CastToBP_FirstPersonCharacter OtherActor))
  (Default|CanopenDoor _asbp_first_person_character true self))

(event OnComponentEndOverlap(Box_N)
  (params (OverlappedComponent :type Primitive%20Component%20Object%20Reference) (OtherActor :type Actor%20Object%20Reference) (OtherComp :type Primitive%20Component%20Object%20Reference) (OtherBodyIndex :type Integer))
  (bind _asbp_first_person_character (Utilities|Casting|CastToBP_FirstPersonCharacter OtherActor))
  (Default|CanopenDoor _asbp_first_person_character false))

(event OnComponentEndOverlap(Box1_N)
  (params (OverlappedComponent :type Primitive%20Component%20Object%20Reference) (OtherActor :type Actor%20Object%20Reference) (OtherComp :type Primitive%20Component%20Object%20Reference) (OtherBodyIndex :type Integer))
  (bind _asbp_first_person_character (Utilities|Casting|CastToBP_FirstPersonCharacter OtherActor))
  (Default|CanopenDoor _asbp_first_person_character false))

(event Custom|OpenDoor
  (params (OpenDoor :type Boolean))
  (if (not (Variables|Default|GetDoorisCurrentlyOpening))
    (Variables|Default|SetDoorisCurrentlyOpening false)
    (bind _output_get (Variables|Default|SetOpendoor_0 OpenDoor))
    (if _output_get
      (Variables|Default|Setdooropeningtemp (Variables|Default|GetDooropeningRotator))
      (bind _door_opening_ (Timeline|DoorOpeningAnimation PlayFromStart)
        (:Update
          _)
        (:Finished
          (Variables|Default|SetDoorisCurrentlyOpening false)))
      (Transformation|SetWorldRotation (Variables|Default|GetDoor_N) (Math|Rotator|Lerp(Rotator) "0, 0, 0" (Variables|Default|Getdooropeningtemp) _door_opening_) false false)
      (else
        (Timeline|DoorOpeningAnimation ReverseFromEnd)))))

(fn ConstructionScript)