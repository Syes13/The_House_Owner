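; BP_Door_2 is a hinged mansion door that the first-person character can open and close from either of two trigger boxes.
; Each box shows its widget and passes the door to the character through CanopenDoor, clearing both on exit.
; OpenDoor plays or reverses a Timeline that lerps the door's world rotation from zero to the same target for both boxes.
; Its DoorisCurrentlyOpening guard is never set true, so it never blocks calls.
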(event OnComponentBeginOverlap(Box_1_E)
  (params (OverlappedComponent :type Primitive%20Component%20Object%20Reference) (OtherActor :type Actor%20Object%20Reference) (OtherComp :type Primitive%20Component%20Object%20Reference) (OtherBodyIndex :type Integer) (bFromSweep :type Boolean) (SweepResult :type Hit%20Result%20Structure%20%28by%20ref%29))
  (Variables|Default|SetDooropeningRotator "0.000000,90.000000,0.000000")
  (bind _asbp_first_person_character (Utilities|Casting|CastToBP_FirstPersonCharacter OtherActor))
  (Default|CanopenDoor _asbp_first_person_character true 0 self)
  (Rendering|SetVisibility (Variables|Default|GetWidget) true false))

(event OnComponentEndOverlap(Box_1_E)
  (params (OverlappedComponent :type Primitive%20Component%20Object%20Reference) (OtherActor :type Actor%20Object%20Reference) (OtherComp :type Primitive%20Component%20Object%20Reference) (OtherBodyIndex :type Integer))
  (bind _asbp_first_person_character (Utilities|Casting|CastToBP_FirstPersonCharacter OtherActor))
  (Default|CanopenDoor _asbp_first_person_character false)
  (Rendering|SetVisibility (Variables|Default|GetWidget) false false))

(event OnComponentBeginOverlap(Box_2_E)
  (params (OverlappedComponent :type Primitive%20Component%20Object%20Reference) (OtherActor :type Actor%20Object%20Reference) (OtherComp :type Primitive%20Component%20Object%20Reference) (OtherBodyIndex :type Integer) (bFromSweep :type Boolean) (SweepResult :type Hit%20Result%20Structure%20%28by%20ref%29))
  (Variables|Default|SetDooropeningRotator "0.000000,90.000000,0.000000")
  (bind _asbp_first_person_character (Utilities|Casting|CastToBP_FirstPersonCharacter OtherActor))
  (Default|CanopenDoor _asbp_first_person_character true 0 self)
  (Rendering|SetVisibility (Variables|Default|GetWidget1) true false))

(event OnComponentEndOverlap(Box_2_E)
  (params (OverlappedComponent :type Primitive%20Component%20Object%20Reference) (OtherActor :type Actor%20Object%20Reference) (OtherComp :type Primitive%20Component%20Object%20Reference) (OtherBodyIndex :type Integer))
  (bind _asbp_first_person_character (Utilities|Casting|CastToBP_FirstPersonCharacter OtherActor))
  (Default|CanopenDoor _asbp_first_person_character false)
  (Rendering|SetVisibility (Variables|Default|GetWidget1) false false))

(event Custom|OpenDoor
  (params (Opendoor :type Boolean))
  (if (not (Variables|Default|GetDoorisCurrentlyOpening))
    (Variables|Default|SetDoorisCurrentlyOpening false)
    (bind _output_get (Variables|Default|SetOpendoor_0 Opendoor))
    (if _output_get
      (Variables|Default|Setdooropeningtemp (Variables|Default|GetDooropeningRotator))
      (bind _door_opening_ (Timeline|Timeline PlayFromStart)
        (:Update
          _)
        (:Finished
          (Variables|Default|SetDoorisCurrentlyOpening false)))
      (Transformation|SetWorldRotation (Variables|Default|GetDoor_E) (Math|Rotator|Lerp(Rotator) "0, 0, 0" (Variables|Default|Getdooropeningtemp) _door_opening_) false false)
      (else
        (Timeline|Timeline ReverseFromEnd)))))

(fn ConstructionScript)